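; Tower projectile Blueprint that homes in on a target enemy and damages it on contact.
; Each tick it moves toward the Targetenemy location at constant speed using VInterpToConstant, without sweeping.
; Its Sphere overlap applies damage only when the overlapping actor is that target, then destroys the projectile.
; The graph neither sets Targetenemy nor checks that it is still valid.
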(event `self.ReceiveTick`
  (params (DeltaSeconds :type "Float (single-precision)"))
  (`self.K2_SetActorLocation` (`KismetMathLibrary.VInterpTo_Constant` (`self.K2_GetActorLocation`) (`self.K2_GetActorLocation` (`self.targetenemy`)) DeltaSeconds 500.0)))

(event `self.Sphere.OnComponentBeginOverlap`
  (params (OverlappedComponent :type "PrimitiveComponent Object Reference") (OtherActor :type "Actor Object Reference") (OtherComp :type "PrimitiveComponent Object Reference") (OtherBodyIndex :type Integer) (bFromSweep :type Boolean) (SweepResult :type "HitResult Structure (by ref)"))
  (bind _targetenemy (`self.targetenemy`))
  (if (== _targetenemy OtherActor)
    (`GameplayStatics.ApplyDamage` _targetenemy 1.0)
    (`self.K2_DestroyActor`)))

(fn `UserConstructionScript`)