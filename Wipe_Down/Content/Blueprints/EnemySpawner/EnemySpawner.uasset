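; Wave spawner actor that alternates preparation time with enemy waves, reading and updating counts on WipeDownGameMode.
; Tick spawns a full wave once the preparation timer expires, then calls NextWave when the enemy count reaches zero.
; SpawnEnemy cycles through two basic enemies and one tank from object pools.
; Each is placed at a random direction and fixed radius around the spawner, with ScatEnemy health reset to max.
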(event `self.ReceiveBeginPlay`
  (bind _aswipe_down_game_mode (cast `WipeDownGameMode` (`GameplayStatics.GetGameMode`)))
  (set `self.GameMode` _aswipe_down_game_mode))

(event `self.ReceiveTick`
  (params (DeltaSeconds :type "Float (single-precision)"))
  (if (`self.WaveOngoing`)
    (bind _returnvalue (`WipeDownGameMode.GetNumberOfEnemies` (`self.GameMode`)))
    (if (<= _returnvalue 0)
      (set `self.WaveOngoing` false)
      (set `self.CurrentWaveTimePreparation` 0.0)
      (`WipeDownGameMode.NextWave` (`self.GameMode`)))
    (else
      (bind _output_get (set `self.CurrentWaveTimePreparation` (+ DeltaSeconds (`self.CurrentWaveTimePreparation`))))
      (if (> _output_get (`self.WaveTimePreparation`))
        (set `self.WaveOngoing` true)
        (bind _returnvalue_2 (`WipeDownGameMode.GetMaxEnemies` (`self.GameMode`)))
        (bind _result (`/Engine/EditorBlueprintResources/StandardMacros.DecrementInt` _returnvalue_2)
          (:`  `
            (for _ (range (+ _result 1))
              (`self.SpawnEnemy`)
              (`/Engine/EditorBlueprintResources/StandardMacros.IncrementInt` (`self.EnemyCount`)))
            (bind _returnvalue_3 (`WipeDownGameMode.GetMaxEnemies` (`self.GameMode`)))
            (`WipeDownGameMode.SetNumberOfEnemies` (`self.GameMode`) _returnvalue_3)))))))

(fn `SpawnEnemy`
  (bind _returnvalue (`KismetMathLibrary.DegreesToRadians` (`KismetMathLibrary.RandomFloatInRange` 0.0 360.0)))
  (bind _returnvalue_2 (+ (* (`KismetMathLibrary.Normal` (`KismetMathLibrary.MakeVector` (`KismetMathLibrary.Sin` _returnvalue) (`KismetMathLibrary.Cos` _returnvalue))) 3000.0) (`self.K2_GetActorLocation`)))
  (switch `int` (mod (`self.EnemyCount`) 3)
    (:`0`
      (bind _returnvalue_3 (`ObjectPoolCharacter.RequestPoolable` (`self.BasicEnemyObjectPool`)))
      (`self.K2_SetActorLocation` _returnvalue_3 _returnvalue_2 false false)
      (bind _asscat_enemy (cast `ScatEnemy` _returnvalue_3))
      (set `ScatEnemy.currentHealth` (`ScatEnemy.maxHealth` _asscat_enemy) _asscat_enemy))
    (:`1`
      (bind _returnvalue_4 (`ObjectPoolCharacter.RequestPoolable` (`self.BasicEnemyObjectPool`)))
      (`self.K2_SetActorLocation` _returnvalue_4 _returnvalue_2 false false)
      (bind _asscat_enemy_2 (cast `ScatEnemy` _returnvalue_4))
      (set `ScatEnemy.currentHealth` (`ScatEnemy.maxHealth` _asscat_enemy_2) _asscat_enemy_2))
    (:`2`
      (bind _returnvalue_5 (`ObjectPoolCharacter.RequestPoolable` (`self.TankEnemyObjectPool`)))
      (`self.K2_SetActorLocation` _returnvalue_5 _returnvalue_2 false false)
      (bind _asscat_enemy_3 (cast `ScatEnemy` _returnvalue_5))
      (set `ScatEnemy.currentHealth` (`ScatEnemy.maxHealth` _asscat_enemy_3) _asscat_enemy_3))))

(fn `UserConstructionScript`)