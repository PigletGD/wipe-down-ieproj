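; HolySeatOld_BP is a damageable objective that earns the player money and ends the game when destroyed.
; On BeginPlay it fills its health and adds a health bar widget to the viewport.
; Tick accumulates time and pays money into WipeDownGameInstance at each generation interval, carrying the remainder over.
; TakeDamage lowers health until zero, then hides the mesh, shows the game-over widget and pauses the game.
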(event `self.ReceiveBeginPlay`
  (set `self.CurrentHealth` (`self.MaxHealth`))
  (bind _returnvalue (`|CreateWidget` "/Game/UI/HealthBar_UI.HealthBar_UI_C"))
  (bind _output_get (set `self.HealthBar_UI` _returnvalue))
  (`UserWidget.AddToViewport` _output_get 0))

(event `self.ReceiveTick`
  (params (DeltaSeconds :type "Float (single-precision)"))
  (bind _output_get (set `self.CurrentGenerationTime` (+ DeltaSeconds (`self.CurrentGenerationTime`))))
  (if (> _output_get (`self.GenerationTime`))
    (set `self.CurrentGenerationTime` (- (`self.CurrentGenerationTime`) (`self.GenerationTime`)))
    (bind _aswipe_down_game_instance (cast `WipeDownGameInstance` (`GameplayStatics.GetGameInstance`)))
    (`WipeDownGameInstance.AddMoney` _aswipe_down_game_instance (`self.MoneyGenerated`))))

(fn `TakeDamage`
  (params (Damage :type Integer))
  (if (not (`self.GameOver`))
    (bind _output_get (set `self.CurrentHealth` (- (`self.CurrentHealth`) Damage)))
    (if (<= _output_get 0)
      (`SceneComponent.SetVisibility` (`self.StaticMesh`) false false)
      (set `self.GameOver` true)
      (bind _returnvalue (`|CreateWidget` "/Game/UI/GameOver_UI.GameOver_UI_C"))
      (`UserWidget.AddToViewport` _returnvalue 0)
      (`GameplayStatics.SetGamePaused` true))))

(fn `UserConstructionScript`)