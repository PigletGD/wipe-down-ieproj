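; Placeable defensive tower that costs money from WipeDownGameInstance when it spawns and automatically shoots at nearby enemies.
; A sphere overlap maintains a list of Enemy targets and switches firing on while any remain in range.
; Tick accumulates time against FireRate, then spawns a Towerproj aimed at the oldest listed target.
; TakeDamage lowers health, starting from MaxHealth, and destroys the tower when it runs out.
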(event `self.ReceiveBeginPlay`
  (bind _aswipe_down_game_instance (cast `/Game/Blueprints/WipeDownGameInstance` (`GameplayStatics.GetGameInstance`)))
  (`/Game/Blueprints/WipeDownGameInstance.SpendMoney` _aswipe_down_game_instance 10)
  (set `self.CurrentHealth` (`self.MaxHealth`)))

(event `self.ReceiveTick`
  (params (DeltaSeconds :type "Float (single-precision)"))
  (bind _output_get (set `self.CurrentFireTick` (+ DeltaSeconds (`self.CurrentFireTick`))))
  (if (and (`self.Fire`) (> _output_get (`self.FireRate`)))
    (`self.FireBullet` (`|GetArrayItem` (`self.Target`)))
    (set `self.CurrentFireTick` 0.0)))

(event `self.sphere.OnComponentBeginOverlap`
  (params (OverlappedComponent :type "PrimitiveComponent Object Reference") (OtherActor :type "Actor Object Reference") (OtherComp :type "PrimitiveComponent Object Reference") (OtherBodyIndex :type Integer) (bFromSweep :type Boolean) (SweepResult :type "HitResult Structure (by ref)"))
  (bind _asenemy (cast `/Game/AI/NPC/Enemy` OtherActor))
  (`KismetArrayLibrary.Array_AddUnique` (`self.Target`) _asenemy)
  (set `self.Fire` true))

(event `self.sphere.OnComponentEndOverlap`
  (params (OverlappedComponent :type "PrimitiveComponent Object Reference") (OtherActor :type "Actor Object Reference") (OtherComp :type "PrimitiveComponent Object Reference") (OtherBodyIndex :type Integer))
  (bind _asenemy (cast `/Game/AI/NPC/Enemy` OtherActor))
  (`KismetArrayLibrary.Array_RemoveItem` (`self.Target`) _asenemy)
  (if (<= (`KismetArrayLibrary.Array_Length` (`self.Target`)) 0)
    (set `self.Fire` false)))

(fn `FireBullet`
  (params (targetenemy :type "/Game/AI/NPC/Enemy Object Reference"))
  (`|SpawnActorFromClass` "/Game/Blueprints/towerproj.towerproj_C" (`self.GetTransform`) "AlwaysSpawn" "OverrideRootScale" null targetenemy null))

(fn `TakeDamage`
  (params (Damage :type Integer))
  (set `self.CurrentHealth` (- (`self.CurrentHealth`) Damage))
  (if (<= (`self.CurrentHealth`) 0)
    (`self.K2_DestroyActor`)))

(fn `UserConstructionScript`)